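; BP_WinPainting is a pickup painting that wins the game for the player who picks it up.
; Overlapping its PickupTrigger calls TryToPickUp on the player character, and its Pickup event destroys the painting and calls YouWin on the parent mesh's owner.
; It also implements Drop, which detaches it into physics, and a PrimaryAction that prints a placeholder health message, clears HeldItem and destroys it.
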(event OnComponentBeginOverlap(PickupTrigger)
  (params (OverlappedComponent :type Primitive%20Component%20Object%20Reference) (OtherActor :type Actor%20Object%20Reference) (OtherComp :type Primitive%20Component%20Object%20Reference) (OtherBodyIndex :type Integer) (bFromSweep :type Boolean) (SweepResult :type Hit%20Result%20Structure%20%28by%20ref%29))
  (bind _asbp_third_person_character_custom (Utilities|Casting|CastToBP_ThirdPersonCharacterCustom OtherActor))
  (Default|TrytoPickUp _asbp_third_person_character_custom self))

(event EventPickup
  (params (ParentMesh :type Skeletal%20Mesh%20Component%20Object%20Reference))
  (Actor|DestroyActor)
  (bind _asbp_third_person_character_custom (Utilities|Casting|CastToBP_ThirdPersonCharacterCustom (Components|GetOwner ParentMesh)))
  (Default|YouWin _asbp_third_person_character_custom))

(event EventDrop
  (bind _painting (Variables|Default|GetPainting))
  (Variables|Default|SetDrop%20Location (Transformation|GetWorldLocation _painting))
  (Transformation|DetachFromComponent _painting "KeepRelative" "KeepRelative" "KeepRelative" true) ; Don't follow the hand anymore
  (Physics|SetSimulatePhysics (Variables|Default|GetPainting) true) ; use gravity to fall
  (Collision|SetCollisionEnabled (Variables|Default|GetPainting) "QueryAndPhysics") ; Collide with the ground please
  (Transformation|SetWorldLocation (Variables|Default|GetPainting) (Variables|Default|GetDrop%20Location) false false) ; To prevent the can from going to world origin
)

(event EventPrimaryAction
  (params (ref_thirdPersonChar :type BP%20Third%20Person%20Character%20Custom%20Object%20Reference))
  ;[1 1 1] Comment
  (Development|PrintString "+10 health!") ; TODO: Implement a health system.
  (Variables|/Game/StealthGame/Core/Characters/PlayerCharacter/BP_ThirdPersonCharacterCustom.BP_ThirdPersonCharacterCustom_C|SetHeldItem ref_thirdPersonChar 0) ; Set the player's held item to nothing
  (Actor|DestroyActor) ; destroy this item
)

(fn ConstructionScript)