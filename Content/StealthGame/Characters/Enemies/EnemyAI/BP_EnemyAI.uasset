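; Stealth-game enemy that patrols, chases the player on sight and investigates thrown distraction items.
; Tick chases while PlayerVisible, otherwise starts a move to the next looping patrol point with randomized speed and pause whenever CanMove allows.
; PawnSensing sight sets PlayerVisible and a retriggerable delay clears it shortly after sightings stop; hearing a BP_DistractionItemPawn sends the enemy to that item's path end.
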(event OnSeePawn(PawnSensing)
  (params (Pawn :type Pawn%20Object%20Reference))
  (Utilities|FlowControl|Sequence
    (:then_0
      (Utilities|Casting|CastToBP_ThirdPersonCharacterStealth Pawn
        (:then
          (Development|PrintString "I see you :D")
          (Variables|Default|SetbPlayerVisible true)
          (CallFunction|ChasePlayer))
        (:CastFailed
          (Variables|Default|SetbPlayerVisible false))))
    (:then_1
      (Utilities|FlowControl|RetriggerableDelay 0.2)
      (Development|PrintString "Hmm next time")
      (Variables|Default|SetbPlayerVisible false))))

(event OnHearNoise(PawnSensing)
  (params (Instigator :type Pawn%20Object%20Reference) (Location :type Vector%20%28by%20ref%29 :default "0, 0, 0") (Volume :type Float%20%28single-precision%29))
  (bind _asbp_distraction_item_pawn (Utilities|Casting|CastToBP_DistractionItemPawn Instigator))
  (CallFunction|UpdateWalkSpeed 2e+02)
  (Variables|Default|SetbCanMove false)
  (AI|AIMoveTo self (Variables|/Game/StealthGame/Gadgets/NoiseMakers/BP_DistractionItemPawn.BP_DistractionItemPawn_C|GetPathEndLocation _asbp_distraction_item_pawn) 0 5.0 false
    (:OnSuccess
      _)
    (:OnFail
      _))
  (Utilities|FlowControl|Delay 2.0)
  (Variables|Default|SetbCanMove true))

(event Custom|ChasePlayer
  (CallFunction|UpdateWalkSpeed 6e+02)
  (Variables|Default|SetbCanMove false)
  (AI|AIMoveTo self "0, 0, 0" (Game|GetPlayerCharacter 0) 5.0 false))

(event Custom|PawnPatrol
  (CallFunction|UpdateWalkSpeed 2e+02)
  (Variables|Default|SetbCanMove false)
  (AI|AIMoveTo self (.RandomLocation (AI|Navigation|GetRandomReachablePointinRadius (Transformation|GetActorLocation) 0.0 0 0)) 0 5.0 false
    (:OnSuccess
      _)
    (:OnFail
      _))
  (Utilities|FlowControl|Delay 2.0)
  (Variables|Default|SetbCanMove true))

(event Custom|MoveToNextPatrolPoint
  (bind _returnvalue (Math|Random|RandomFloatinRange 1.5 5.0))
  (CallFunction|UpdateWalkSpeed (Math|Random|RandomFloatinRange 175.0 2.5e+02))
  (Variables|Default|SetbCanMove false)
  (AI|AIMoveTo self "0, 0, 0" (Utilities|Array|Get(acopy) (Variables|Default|GetPatrolTargetPoints) (Variables|Default|GetPatrolTargetPointIndex)) 5.0 false
    (:OnSuccess
      (Utilities|FlowControl|Delay _returnvalue)
      (Variables|Default|SetbCanMove true)
      (CallFunction|SetNextPatrolIndex))
    (:OnFail
      (Utilities|FlowControl|Delay _returnvalue)
      (Variables|Default|SetbCanMove true))))

(event Custom|SetNextPatrolIndex
  (Variables|Default|SetPatrolTargetPointIndex (Math|Integer|%(Integer) (+ (Variables|Default|GetPatrolTargetPointIndex) 1) (Utilities|Array|Length (Variables|Default|GetPatrolTargetPoints)))))

(event EventBeginPlay)

(event Collision|EventActorBeginOverlap
  (params (OtherActor :type Actor%20Object%20Reference)))

(event EventTick
  (params (DeltaSeconds :type Float%20%28single-precision%29))
  (bind _bplayervisible (Variables|Default|GetbPlayerVisible))
  ;[0.15 0.15 0.15 0.5] hold b and left click for branch node
  (if (Variables|Default|GetbCanMove)
    (if _bplayervisible
      (CallFunction|ChasePlayer :!label _label)
      (else
        (CallFunction|MovetoNextPatrolPoint)))
    (else
      ;[0.15 0.007243 0.01185 0.5] if you cant move but see the player chase
      (if _bplayervisible
        (goto _label)))))

(fn ConstructionScript)

(fn UpdateWalkSpeed
  (params (Walk%20Speed :type Float%20%28double-precision%29))
  (Variables|/Script/Engine.CharacterMovementComponent|SetMaxWalkSpeed (Variables|Character|GetCharacterMovement) Walk%20Speed))